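; BP_MovingEnemy is an enemy that chases the player and can be killed by damage.
; On BeginPlay it issues a single AI MoveTo targeting the player's BP_FirstPersonCharacter.
; AnyDamage subtracts from Health; at zero or below, the enemy calls KillTarget on that character with a value of 2, then destroys itself.
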(event EventBeginPlay
  (bind _asbp_first_person_character (Utilities|Casting|CastToBP_FirstPersonCharacter (Game|GetPlayerCharacter 0)))
  (Utilities|FlowControl|Sequence
    (:then_0
      (AI|AIMoveTo self "0, 0, 0" _asbp_first_person_character 5.0 false))))

(event Collision|EventActorBeginOverlap
  (params (OtherActor :type Actor%20Object%20Reference)))

(event EventTick
  (params (DeltaSeconds :type Float%20%28single-precision%29)))

(event Game|Damage|EventAnyDamage
  (params (Damage :type Float%20%28single-precision%29) (DamageType :type Damage%20Type%20Object%20Reference) (InstigatedBy :type Controller%20Object%20Reference) (DamageCauser :type Actor%20Object%20Reference))
  (Variables|Default|SetHealth (- (Variables|Default|GetHealth) Damage))
  (if (<= (Variables|Default|GetHealth) 0.0)
    (Utilities|FlowControl|Sequence
      (:then_0
        (bind _asbp_first_person_character (Utilities|Casting|CastToBP_FirstPersonCharacter (Game|GetPlayerCharacter 0)))
        (Variables|Default|SetAs%20BP%20First%20Person%20Character _asbp_first_person_character))
      (:then_1
        (Default|KillTarget (Variables|Default|GetAs%20BP%20First%20Person%20Character) 2)
        (Actor|DestroyActor)))))

(fn ConstructionScript)